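; Game mode for a timed statue-collecting game that opens on a paused main menu and handles game over and a saved leaderboard.
; A Delay on Tick drives a one-second countdown, while each collected statue adds time and level-based points.
; MoveStatue spawns a statue at a random BP_SpawnPoint.
; When time expires, GameOver pauses play and appends name and score to the LB save slot, which DrawLB displays.
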(event `self.ReceiveBeginPlay`
  (`self.MainMenu`))

(event `self.ReceiveTick`
  (params (DeltaSeconds :type "Float (single-precision)"))
  (`KismetSystemLibrary.Delay` 1.0)
  (`self.Timer`))

(fn `DrawLB`
  (bind _mylbsave (`self.MyLBSave`))
  (bind _returnvalue (`|CreateWidget` "/Game/Leaderboard.Leaderboard_C"))
  (`UserWidget.SetAlignmentInViewport` _returnvalue (0.5 0.5))
  (`UserWidget.SetAnchorsInViewport` _returnvalue (make `Anchors` (0.5 0.5) (0.5 0.5)))
  (`UserWidget.SetPositionInViewport` _returnvalue (/ (`WidgetLayoutLibrary.GetViewportSize`) 2.0) true)
  (`UserWidget.SetDesiredSizeInViewport` _returnvalue (500.0 800.0))
  (`UserWidget.AddToViewport` _returnvalue 0)
  (`/Game/Leaderboard.AddData` _returnvalue (`/Game/LB_SaveData.PlayerNames` _mylbsave) (`/Game/LB_SaveData.PlayerScores` _mylbsave)))

(fn `GameOver`
  (bind _returnvalue (`GameplayStatics.GetPlayerController` 0))
  (bind _returnvalue_2 (`|CreateWidget` "/Game/GameOver.GameOver_C"))
  (`UserWidget.AddToViewport` _returnvalue_2 0)
  (`self.DisableInput` (`GameplayStatics.GetPlayerCharacter` 0) _returnvalue)
  (set `PlayerController.bShowMouseCursor` true _returnvalue)
  (`GameplayStatics.SetGamePaused` true)
  (`self.SetLB`))

(fn `MainMenu`
  (bind _returnvalue (`GameplayStatics.GetPlayerController` 0))
  (bind _returnvalue_2 (`|CreateWidget` "/Game/Menu.Menu_C"))
  (bind _output_get (set `self.MenuWidget` _returnvalue_2))
  (`UserWidget.AddToViewport` _output_get 0)
  (`GameplayStatics.SetGamePaused` true)
  (`self.DisableInput` (`GameplayStatics.GetPlayerCharacter` 0) _returnvalue)
  (set `PlayerController.bShowMouseCursor` true _returnvalue))

(fn `MoveStatue`
  (bind _outactors (`GameplayStatics.GetAllActorsOfClass` "/Game/BP_SpawnPoint.BP_SpawnPoint_C"))
  (`|SpawnActorFromClass` "/Game/Bp_Statue.BP_Statue_C" (`self.GetTransform` (`|GetArrayItem` _outactors (`KismetMathLibrary.RandomIntegerInRange` 0 (`KismetArrayLibrary.Array_LastIndex` _outactors)))) "Undefined" "OverrideRootScale" null null))

(fn `SetLB`
  (bind _returnvalue (`GameplayStatics.DoesSaveGameExist` "LB"))
  (if _returnvalue
    (bind _returnvalue_2 (`GameplayStatics.LoadGameFromSlot` "LB"))
    (bind _aslb_save_data (cast `/Game/LB_SaveData` _returnvalue_2))
    (bind _output_get (set `self.MyLBSave` _aslb_save_data))
    (if (> (`self.Score`) 0)
      (`KismetArrayLibrary.Array_Add` (`/Game/LB_SaveData.PlayerNames` _output_get) (`self.MyName`))
      (`KismetArrayLibrary.Array_Add` (`/Game/LB_SaveData.PlayerScores` _output_get) (`self.Score`))
      (`GameplayStatics.SaveGameToSlot` (`self.MyLBSave`) "LB"))
    (else
      (bind _returnvalue_3 (`GameplayStatics.CreateSaveGameObject` "/Game/LB_SaveData.LB_SaveData_C"))
      (bind _output_get_2 (set `self.MyLBSave` _returnvalue_3))
      (if (> (`self.Score`) 0)
        (`KismetArrayLibrary.Array_Add` (`/Game/LB_SaveData.PlayerNames` _output_get_2) (`self.MyName`))
        (`KismetArrayLibrary.Array_Add` (`/Game/LB_SaveData.PlayerScores` _output_get_2) (`self.Score`))
        (`GameplayStatics.SaveGameToSlot` (`self.MyLBSave`) "LB")))))

(fn `Statue Collected`
  (if (`KismetStringLibrary.EqualEqual_StrStr` (`self.Level`) "1")
    (set `self.Time` (+ (`self.Time`) 4))
    (set `self.Score` (+ (`self.Score`) 10))
    (set `self.StatueCollected` (+ (`self.StatueCollected`) 1))
    (elif (`KismetStringLibrary.EqualEqual_StrStr` (`self.Level`) "2")
      (set `self.Time` (+ (`self.Time`) 4))
      (set `self.Score` (+ (`self.Score`) 20))
      (set `self.StatueCollected` (+ (`self.StatueCollected`) 1))
      (elif (`KismetStringLibrary.EqualEqual_StrStr` (`self.Level`) "3")
        (set `self.Time` (+ (`self.Time`) 4))
        (set `self.Score` (+ (`self.Score`) 30))
        (set `self.StatueCollected` (+ (`self.StatueCollected`) 1))
        (elif (`KismetStringLibrary.EqualEqual_StrStr` (`self.Level`) "max")
          (set `self.Time` (+ (`self.Time`) 4))
          (set `self.Score` (+ (`self.Score`) 40))
          (set `self.StatueCollected` (+ (`self.StatueCollected`) 1)))))))

(fn `Timer`
  (if (> (`self.Time`) 0)
    (bind _output_get (set `self.Time` (+ (`self.Time`) -1)))
    (if (<= _output_get 0)
      (`self.GameOver`))))

(fn `UserConstructionScript`)